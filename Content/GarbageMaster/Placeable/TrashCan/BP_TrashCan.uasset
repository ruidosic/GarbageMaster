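; BP_TrashCan is a placeable trash can that notifies a BP_Vehicle on overlap to grab its garbage.
; Timelines tilt the cap and body, with the body tilt triggering a one-time, delayed-loop spawn of physics-simulated trash packages.
; A separate hit event launches the body with physics impulses.
; When movable, it follows touch drags via screen-to-world traces, keeping its initial height.
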(event Custom|CapAnimation
  (bind _trashcancap (Variables|Default|GetTrashCanCap))
  (bind _returnvalue (Transformation|GetWorldRotation _trashcancap))
  (bind (_roll _pitch _yaw) (Math|Rotator|BreakRotator _returnvalue))
  (bind _alpha (Timeline|Animation PlayFromStart)
    (:Update
      (Transformation|SetWorldRotation (Variables|Default|GetTrashCanCap) (Math|Rotator|Lerp(Rotator) _returnvalue (Math|Rotator|MakeRotator -9e+01 _pitch _yaw) _alpha) false false))))

(event Custom|BodyAnimation
  (bind _trashcanbody (Variables|Default|GetTrashCanBody))
  (bind _returnvalue (Transformation|GetWorldRotation _trashcanbody))
  (bind (_roll _pitch _yaw) (Math|Rotator|BreakRotator _returnvalue))
  (bind _alpha (Timeline|Timeline_0 PlayFromStart)
    (:Update
      (Transformation|SetWorldRotation (Variables|Default|GetTrashCanBody) (Math|Rotator|Lerp(Rotator) _returnvalue (Math|Rotator|MakeRotator 1.2e+02 _pitch _yaw) _alpha) false false)
      (if (> _alpha 0.7)
        (Utilities|FlowControl|DoOnce false
          (:Completed
            (CallFunction|SpawnTrash 1.0)))))))

(event Custom|SpawnTrash
  (params (Delay :type Float%20%28single-precision%29))
  (Utilities|ForLoopwithDelay 1 (Variables|Default|GetTrashCount) Delay
    (:Loop
      (bind _returnvalue (Game|SpawnActorfromClass "/Game/GarbageMaster/Placeable/Trash/BP_TrashPackage.BP_TrashPackage_C" (Math|Transform|MakeTransform (Transformation|GetWorldLocation (Variables|Default|GetScene))) "AlwaysSpawn" 0 0))
      (Physics|SetSimulatePhysics (Variables|/Game/GarbageMaster/Placeable/Trash/BP_Trash.BP_Trash_C|GetTrash _returnvalue) true))))

(event Custom|TrashCanHit
  (bind _trashcanbody (Variables|Default|GetTrashCanBody))
  (Transformation|AddWorldOffset (Variables|Default|GetTrashCanBody) "0, 0,20.000000" false false)
  (Collision|SetCollisionEnabled _trashcanbody "PhysicsOnly")
  (Physics|SetSimulatePhysics _trashcanbody true)
  (Timeline|Timeline_1 PlayFromStart
    (:Update
      (Physics|AddImpulse _trashcanbody "0.000000,-10000.000000,5000.000000" "None" false))))

(event Collision|EventActorBeginOverlap
  (params (OtherActor :type Actor%20Object%20Reference))
  (bind _asbp_vehicle (Utilities|Casting|CastToBP_Vehicle OtherActor))
  (Variables|Default|SetMainPawn _asbp_vehicle)
  (Variables|Default|SetTouched false)
  (Collision|SetCollisionEnabled (Variables|Default|GetTrashCanBody) "NoCollision")
  (Default|GrabGarbage _asbp_vehicle self)
  (Default|CallTrashGrabed))

(event EventActorOnInputTouchBegin
  (params (FingerIndex :type ETouchIndex%20Enum :default "Touch1"))
  (if (Variables|Default|GetCanBeMovable)
    (Variables|Default|SetTouched true)))

(event EventActorOnInputTouchEnd
  (params (FingerIndex :type ETouchIndex%20Enum :default "Touch1"))
  (if (Variables|Default|GetCanBeMovable)
    (Variables|Default|SetTouched false)))

(event EventTick
  (params (DeltaSeconds :type Float%20%28single-precision%29))
  (bind _returnvalue (Game|GetPlayerController 0))
  (bind (_locationx _locationy _biscurrentlypressed) (Class|PlayerController|GetInputTouchState _returnvalue "Touch1"))
  (bind _returnvalue_2 (Math|Vector2D|MakeVector2D _locationx _locationy))
  (bind (_worldposition _worlddirection) (Class|GameplayStatics|DeprojectScreentoWorld _returnvalue _returnvalue_2))
  (if (and _biscurrentlypressed (Variables|Default|GetTouched))
    (bind _outhit (Collision|LineTraceByChannel _worldposition (+ _worldposition (* _worlddirection 1e+04)) "TraceTypeQuery1" false 0 "None"))
    (Transformation|SetActorLocation (Math|Vector|MakeVector (.X (Math|Vector|BreakVector (.Location (Collision|BreakHitResult _outhit)))) (.Y (Math|Vector|BreakVector (.Location (Collision|BreakHitResult _outhit)))) (.Z (Math|Vector|BreakVector (Variables|Default|GetBlockZone)))) true false)
    (else
      (Variables|Default|SetTouched false))))

(event EventBeginPlay
  (Variables|Default|SetInitialLocation (Transformation|GetActorLocation))
  (CallFunction|CalculateBlockZone))

(fn ConstructionScript)

(fn GetCapAnimTime
  (return (Components|Timeline|GetTimelineLength (Variables|Default|GetAnimation))))

(fn CalculateBlockZone
  (bind _initiallocation (Variables|Default|GetInitialLocation))
  (bind (_x _y _z) (Math|Vector|BreakVector _initiallocation))
  (Variables|Default|SetBlockZone (Math|Vector|MakeVector (+ (.X (Math|Vector|BreakVector (Variables|Default|GetBlockZone))) _x) (+ (.Y (Math|Vector|BreakVector (Variables|Default|GetBlockZone))) (.Y (Math|Vector|BreakVector (Variables|Default|GetInitialLocation)))) _z)))

(fn SetupTrashCount
  (params (TrashCount :type Integer))
  (Variables|Default|SetTrashCount TrashCount))