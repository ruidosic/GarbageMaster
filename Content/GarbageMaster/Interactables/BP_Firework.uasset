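; BP_Firework is an interactable actor that sets off fireworks when the player pawn first overlaps it.
; A DoOnce gate on the overlap event limits the effect to a single firing.
; It spawns the P_Firework emitter at the world transforms of two components, LeftPoint and RightPoint.
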(event Collision|EventActorBeginOverlap
  (params (OtherActor :type Actor%20Object%20Reference))
  (bind _leftpoint (Variables|Default|GetLeftPoint))
  (bind _rightpoint (Variables|Default|GetRightPoint))
  (bind _returnvalue (Transformation|GetWorldTransform _rightpoint))
  (bind _returnvalue_2 (Transformation|GetWorldTransform _leftpoint))
  (bind (_location _rotation _scale) (Math|Transform|BreakTransform _returnvalue))
  (bind (_location_2 _rotation_2 _scale_2) (Math|Transform|BreakTransform _returnvalue_2))
  (if (== OtherActor (Game|Player|GetPlayerPawn 0))
    (Utilities|FlowControl|DoOnce false
      (:Completed
        (Effects|SpawnEmitteratLocation "/Game/GarbageMaster/Art/Effects/P_Firework.P_Firework" _location_2 _rotation_2 _scale_2)
        (Effects|SpawnEmitteratLocation "/Game/GarbageMaster/Art/Effects/P_Firework.P_Firework" _location _rotation _scale)))))

(fn ConstructionScript)