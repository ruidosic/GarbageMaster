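; BP_InteractableZone is an interactable trigger zone that takes over the player's BP_Vehicle once it slows down inside it.
; Cube overlap starts a looping timer that checks forward speed, and end overlap clears it.
; At low enough speed, it hides the Cube, halts the vehicle, fires the empty InteractableEvent hook and blends the camera to itself.
; SetupCongrats forwards a number to the vehicle's gameplay UI.
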(event OnComponentBeginOverlap(Cube)
  (params (OverlappedComponent :type Primitive%20Component%20Object%20Reference) (OtherActor :type Actor%20Object%20Reference) (OtherComp :type Primitive%20Component%20Object%20Reference) (OtherBodyIndex :type Integer) (bFromSweep :type Boolean) (SweepResult :type Hit%20Result%20Structure%20%28by%20ref%29))
  (bind _asbp_vehicle (Utilities|Casting|CastToBP_Vehicle (Game|Player|GetPlayerPawn 0)))
  (Variables|Default|SetMainPawn _asbp_vehicle)
  (bind _returnvalue (Utilities|Time|SetTimerbyEvent (delegate Custom|CheckSpeed) 0.4 true))
  (Variables|Default|SetCheckSpeedTimer _returnvalue))

(event OnComponentEndOverlap(Cube)
  (params (OverlappedComponent :type Primitive%20Component%20Object%20Reference) (OtherActor :type Actor%20Object%20Reference) (OtherComp :type Primitive%20Component%20Object%20Reference) (OtherBodyIndex :type Integer))
  (Utilities|Time|ClearandInvalidateTimerbyHandle (Variables|Default|GetCheckSpeedTimer)))

(event Custom|CheckSpeed
  (if (Math|Float|InRange(Float) (Class|WheeledVehicleMovementComponent|GetForwardSpeed (Variables|/Script/PhysXVehicles.WheeledVehicle|GetVehicleMovement (Variables|Default|GetMainPawn))) 0.0 4e+02)
    (Rendering|SetVisibility (Variables|Default|GetCube) false false)
    (Default|StopInput (Variables|Default|GetMainPawn))
    (Default|StopMovement (Variables|Default|GetMainPawn))
    (CallFunction|InteractableEvent)
    (Utilities|Time|ClearandInvalidateTimerbyHandle (Variables|Default|GetCheckSpeedTimer))
    (Game|Player|SetViewTargetwithBlend (Game|GetPlayerController 0) self 1.0 "VTBlend_Linear" 0.0 false)))

(event Custom|InteractableEvent)

(event Custom|SetupCongrats
  (params (CongratNumber :type Integer))
  (Default|SetupText (Variables|/Game/GarbageMaster/Vehicle/MainVehicle/Blueprints/BP_Vehicle.BP_Vehicle_C|GetGameplayUI (Variables|Default|GetMainPawn)) CongratNumber))

(fn ConstructionScript)