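; BP_ThrashZone is an interactable trash zone that rates how close the player is to it and enables moving its child-actor trash can.
; BeginPlay passes TrashCount to the can and binds its grab event to an empty CameraZoom.
; Interaction converts X-axis distance from the Cube into a congrats tier, calls SetupCongrats, makes the can movable and repositions the camera relative to the player.
; The zoom timeline is never triggered.
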(event Custom|CameraZoom)

(event Custom|MoveTrashCan
  (Variables|/Game/GarbageMaster/Placeable/TrashCan/BP_TrashCan.BP_TrashCan_C|SetCanBeMovable (Variables|Default|GetThrashCan) true))

(event EventInteractableEvent
  (bind _camera (Variables|Default|GetCamera))
  (CallFunction|CalculateCongratNumber)
  (CallFunction|SetupCongrats (Variables|Default|GetCongratNumber))
  (CallFunction|MoveTrashCan)
  (Transformation|SetWorldLocation _camera (+ (Variables|/Script/Engine.SceneComponent|GetRelativeLocation _camera) (Transformation|GetActorLocation (Game|Player|GetPlayerPawn 0))) false false))

(event EventBeginPlay
  (bind _asbp_trash_can (Utilities|Casting|CastToBP_TrashCan (Variables|/Script/Engine.ChildActorComponent|GetChildActor (Variables|Default|GetTrashCanActor))))
  (bind _output_get (Variables|Default|SetThrashCan _asbp_trash_can))
  (Default|SetupTrashCount _output_get (Variables|Default|GetTrashCount))
  (EventDispatchers|BindEventtoTrashGrabed (Variables|Default|GetThrashCan) (delegate Custom|CameraZoom)))

(fn ConstructionScript)

(fn DistancefromZonetoPlayer
  (return (.X (Math|Vector|BreakVector (Math|Vector|VectorGetAbs (- (Transformation|GetActorLocation (Game|Player|GetPlayerPawn 0)) (Transformation|GetWorldLocation (Variables|Default|GetCube))))))))

(fn CalculateCongratNumber
  (bind _distance (CallFunction|DistancefromZonetoPlayer))
  (if (Math|Float|InRange(Float) _distance 0.0 1e+02 true false)
    (Variables|Default|SetCongratNumber 2)
    (elif (Math|Float|InRange(Float) _distance 1e+02 2e+02)
      (Variables|Default|SetCongratNumber 1)
      (elif (Math|Float|InRange(Float) _distance 2e+02 3e+02 false)
        (Variables|Default|SetCongratNumber 0)))))