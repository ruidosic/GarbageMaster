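; BP_Dump is the garbage dump interactable that scores deliveries and ends the level.
; Its TrashDetect overlap counts incoming BP_Trash, while InteractableEvent moves the camera relative to the player and sets the main pawn's body to rotate.
; It binds to the vehicle's finish event, waits briefly, then adds the trash count to GameInstance stars and shows the level-complete widget with that count as the rating.
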(event OnComponentBeginOverlap(TrashDetect)
  (params (OverlappedComponent :type Primitive%20Component%20Object%20Reference) (OtherActor :type Actor%20Object%20Reference) (OtherComp :type Primitive%20Component%20Object%20Reference) (OtherBodyIndex :type Integer) (bFromSweep :type Boolean) (SweepResult :type Hit%20Result%20Structure%20%28by%20ref%29))
  (Utilities|Casting|CastToBP_Trash OtherActor)
  (Math|Integer|IncrementInt (Variables|Default|GetTrashCount)))

(event Custom|CheckGarbage
  (Utilities|FlowControl|Delay 3.0)
  (CallFunction|NextLevel))

(event EventBeginPlay
  (EventDispatchers|BindEventtoFinish (.AsBP%20Vehicle (Utilities|Casting|CastToBP_Vehicle (Game|Player|GetPlayerPawn 0))) (delegate Custom|CheckGarbage)))

(event EventInteractableEvent
  (bind _camera (Variables|Default|GetCamera))
  (Transformation|SetWorldLocation _camera (+ (Variables|/Script/Engine.SceneComponent|GetRelativeLocation _camera) (Transformation|GetActorLocation (Game|Player|GetPlayerPawn 0))) false false)
  (Default|SetRotateBody (Variables|Default|GetMainPawn) true))

(fn ConstructionScript)

(fn NextLevel
  (bind _trashcount (Variables|Default|GetTrashCount))
  (Default|IncreaseStarsCount (Variables|/Game/GarbageMaster/Vehicle/MainVehicle/Blueprints/BP_Vehicle.BP_Vehicle_C|GetGameInstance (Variables|Default|GetMainPawn)) _trashcount)
  (bind _returnvalue (UserInterface|CreateWidget "/Game/GarbageMaster/UI/LevelComplete/WBP_LevelComplete.WBP_LevelComplete_C" 0 _trashcount))
  (UserInterface|Viewport|AddtoViewport _returnvalue 0))