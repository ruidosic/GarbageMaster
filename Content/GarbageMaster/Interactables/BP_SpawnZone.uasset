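; BP_SpawnZone is a one-use trigger volume that spawns a row of trash actors when a BP_BonusVehicle enters it.
; Each TrashArray class spawns along world X at a start offset from the zone, evenly spaced by DistanceBetween, with DistanceHeight as absolute Z.
; The construction script sizes the box from Size, and the zone destroys itself when the vehicle leaves.
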(event OnComponentBeginOverlap(Box)
  (params (OverlappedComponent :type Primitive%20Component%20Object%20Reference) (OtherActor :type Actor%20Object%20Reference) (OtherComp :type Primitive%20Component%20Object%20Reference) (OtherBodyIndex :type Integer) (bFromSweep :type Boolean) (SweepResult :type Hit%20Result%20Structure%20%28by%20ref%29))
  (Utilities|Casting|CastToBP_BonusVehicle OtherActor)
  (CallFunction|SpawnGarbage))

(event OnComponentEndOverlap(Box)
  (params (OverlappedComponent :type Primitive%20Component%20Object%20Reference) (OtherActor :type Actor%20Object%20Reference) (OtherComp :type Primitive%20Component%20Object%20Reference) (OtherBodyIndex :type Integer))
  (Utilities|Casting|CastToBP_BonusVehicle OtherActor)
  (Actor|DestroyActor))

(event Custom|SpawnGarbage
  (for (_array_element _array_index) (Variables|Default|GetTrashArray)
    (Game|SpawnActorfromClass _array_element (Math|Transform|MakeTransform (Math|Vector|MakeVector (.x (+ (Transformation|GetActorLocation) (Math|Vector|MakeVector (+ (Variables|Default|GetSpawnStartPoint) (* _array_index (Variables|Default|GetDistanceBetween))) 0.0 0.0))) 0.0 (Variables|Default|GetDistanceHeight))) "Undefined" 0 0)))

(fn ConstructionScript
  (Components|Box|SetBoxExtent (Variables|Default|GetBox) (Variables|Default|GetSize) true))