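; BP_BonusVehicle is the player vehicle for a garbage-cleaning bonus level, driving at constant throttle while Move is set.
; Holding touch lowers the cleaner and releasing raises it, within a clamped height.
; Overlap triggers destroy trash, while a stone hitting the cleaner stops throttle, drops it as physics debris, detaches the camera arm and opens LevelBase after a delay.
; Possession shows the bonus menu, and CameraAnim blends the spring arm via timeline.
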(event OnComponentBeginOverlap(CleanerDetectTrash)
  (params (OverlappedComponent :type Primitive%20Component%20Object%20Reference) (OtherActor :type Actor%20Object%20Reference) (OtherComp :type Primitive%20Component%20Object%20Reference) (OtherBodyIndex :type Integer) (bFromSweep :type Boolean) (SweepResult :type Hit%20Result%20Structure%20%28by%20ref%29))
  (bind _sm_cleaner (Variables|Default|GetSM_Cleaner))
  (Utilities|Casting|CastToBP_Trash OtherActor
    (:then
      (Actor|DestroyActor OtherActor))
    (:CastFailed
      (Utilities|Casting|CastToBP_Stone OtherActor)
      (Variables|Default|SetMove false)
      (Transformation|DetachFromComponent _sm_cleaner "KeepWorld" "KeepWorld" "KeepRelative" true)
      (Physics|SetSimulatePhysics _sm_cleaner true)
      (CallFunction|LevelLose))))

(event OnComponentBeginOverlap(VehicleDetectTrash)
  (params (OverlappedComponent :type Primitive%20Component%20Object%20Reference) (OtherActor :type Actor%20Object%20Reference) (OtherComp :type Primitive%20Component%20Object%20Reference) (OtherBodyIndex :type Integer) (bFromSweep :type Boolean) (SweepResult :type Hit%20Result%20Structure%20%28by%20ref%29))
  (Utilities|Casting|CastToBP_Trash OtherActor)
  (Actor|DestroyActor OtherActor))

(event Custom|LevelLose
  (Transformation|DetachFromComponent (Variables|Default|GetSpringArm) "KeepWorld" "KeepWorld" "KeepWorld" true)
  (Utilities|FlowControl|Delay 2.0)
  (Game|OpenLevel(byName) "LevelBase"))

(event Custom|CameraAnim
  (bind _springarm (Variables|Default|GetSpringArm))
  (bind _alpha (Timeline|CameraAnimation Play)
    (:Update
      (Transformation|SetRelativeLocation _springarm (Math|Vector|Lerp(Vector) "0.000000,0.000000,90.000000" "431.000000,165.000000,108.000000" _alpha) false false)
      (Transformation|SetRelativeRotation _springarm (Math|Rotator|Lerp(Rotator) "-10.000000,-80.000000, 0" "-25.000000,-45.000000, 0" _alpha true) false false))))

(event EventBeginPlay)

(event EventTick
  (params (DeltaSeconds :type Float%20%28single-precision%29))
  (bind _vehiclemovement (Variables|Default|GetVehicleMovement))
  (if (Variables|Default|GetMove)
    (Class|WheeledVehicleMovementComponent|SetThrottleInput _vehiclemovement 0.7)
    (else
      (Class|WheeledVehicleMovementComponent|SetThrottleInput _vehiclemovement 0.0))))

(event EventPossessed
  (params (NewController :type Controller%20Object%20Reference))
  (Viewport|RemoveAllWidgets)
  (bind _returnvalue (UserInterface|CreateWidget "/Game/GarbageMaster/UI/MainMenu/WBP_BonusLevelMenu.WBP_BonusLevelMenu_C" 0 self))
  (UserInterface|Viewport|AddtoViewport _returnvalue 0))

(event Input|AxisEvents|InputAxisTouchScreen
  (params (AxisValue :type Float%20%28single-precision%29))
  (bind _sm_cleaner (Variables|Default|GetSM_Cleaner))
  (bind _returnvalue (Transformation|GetWorldLocation _sm_cleaner))
  (bind (_x _y _z) (Math|Vector|BreakVector _returnvalue))
  (if (.bIsCurrentlyPressed (Class|PlayerController|GetInputTouchState (Game|GetPlayerController 0) "Touch1"))
    (Transformation|SetWorldLocation (Variables|Default|GetSM_Cleaner) (Math|Vector|MakeVector _x _y (Math|Float|Clamp(Float) (+ _z -1.0) 0.0 6e+01)) false false)
    (else
      (Transformation|SetWorldLocation (Variables|Default|GetSM_Cleaner) (Math|Vector|MakeVector _x _y (Math|Float|Clamp(Float) (+ _z 1.0) 0.0 6e+01)) false false))))

(fn ConstructionScript)